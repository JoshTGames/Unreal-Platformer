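; BP_Player is the player-controlled character Blueprint for the 2D platformer, translating Enhanced Input into movement intent.
; On BeginPlay, SetupInput adds the IMC_GAME mapping context to the owning player controller's input subsystem.
; Move and slide actions write TargetXVelocity and DoSlide, while jump calls HandleJump; none of that movement logic is defined here.
; Each action's Triggered and Completed events share one path, so releases pass through the same logic.
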(event Input|EnhancedActionEvents|EnhancedInputActionIA_Slide
  (params (ActionValue :type Boolean) (ElapsedSeconds :type Float%20%28double-precision%29) (TriggeredSeconds :type Float%20%28double-precision%29) (InputAction :type Input%20Action%20Object%20Reference :default "/Game/2dPlatformer/Input/Actions/IA_Slide.IA_Slide"))
  (:Triggered
    (Variables|Default|SetdoSlide ActionValue :!label _label))
  (:Completed
    (goto _label)))

(event Input|EnhancedActionEvents|EnhancedInputActionIA_NewMove
  (params (ActionValue :type Float%20%28double-precision%29) (ElapsedSeconds :type Float%20%28double-precision%29) (TriggeredSeconds :type Float%20%28double-precision%29) (InputAction :type Input%20Action%20Object%20Reference :default "/Game/2dPlatformer/Input/Actions/IA_NewMove.IA_NewMove"))
  (:Triggered
    (Variables|Default|SettargetXVelocity ActionValue :!label _label))
  (:Completed
    (goto _label)))

(event Input|EnhancedActionEvents|EnhancedInputActionIA_NewJump
  (params (ActionValue :type Boolean) (ElapsedSeconds :type Float%20%28double-precision%29) (TriggeredSeconds :type Float%20%28double-precision%29) (InputAction :type Input%20Action%20Object%20Reference :default "/Game/2dPlatformer/Input/Actions/IA_NewJump.IA_NewJump"))
  (:Triggered
    (CallFunction|HandleJump ActionValue :!label _label))
  (:Completed
    (goto _label)))

(event EventBeginPlay
  (|CallParentFunction)
  (CallFunction|SetupInput))

(event Collision|EventActorBeginOverlap
  (params (OtherActor :type Actor%20Object%20Reference)))

(event EventTick
  (params (DeltaSeconds :type Float%20%28single-precision%29))
  (|CallParentFunction DeltaSeconds) ; This node is disabled and will not be called.\nDrag off pins to build functionality.
)

(fn ConstructionScript
  (|CallParentFunction))

(fn SetupInput
  (bind _asplayer_controller (Utilities|Casting|CastToPlayerController (Pawn|GetController)))
  (Utilities|IsValid (PlayerController|LocalPlayerSubsystems|GetEnhancedInputLocalPlayerSubsystem _asplayer_controller)
    (:Is%20Valid
      (Input|AddMappingContext (PlayerController|LocalPlayerSubsystems|GetEnhancedInputLocalPlayerSubsystem _asplayer_controller) "/Game/2dPlatformer/Input/IMC_GAME.IMC_GAME" 0 "(bIgnoreAllPressedKeysUntilRelease=True,bForceImmediately=False,bNotifyUserSettings=False)"))))