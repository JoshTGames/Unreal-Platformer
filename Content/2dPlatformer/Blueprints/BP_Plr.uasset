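; BP_Plr is the player character for a 2D platformer, with horizontal movement and jumping.
; Enhanced Input adds its mapping context on BeginPlay, stores the move value as a target X velocity, and starts or stops jumps.
; Tick feeds that value into movement input, then picks an idle, move, jump or fall flipbook from velocity.
; The sprite flips by rotation whenever X velocity is not positive, including at rest.
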(event Input|EnhancedActionEvents|EnhancedInputActionIA_NewMove
  (params (ActionValue :type Float%20%28double-precision%29) (ElapsedSeconds :type Float%20%28double-precision%29) (TriggeredSeconds :type Float%20%28double-precision%29) (InputAction :type Input%20Action%20Object%20Reference :default "/Game/2dPlatformer/Input/Actions/IA_NewMove.IA_NewMove"))
  (:Triggered
    (Variables|Default|SettargetXVelocity ActionValue :!label _label))
  (:Completed
    (goto _label)))

(event Input|EnhancedActionEvents|EnhancedInputActionIA_NewJump
  (params (ActionValue :type Boolean) (ElapsedSeconds :type Float%20%28double-precision%29) (TriggeredSeconds :type Float%20%28double-precision%29) (InputAction :type Input%20Action%20Object%20Reference :default "/Game/2dPlatformer/Input/Actions/IA_NewJump.IA_NewJump"))
  (:Triggered
    (Character|Jump))
  (:Completed
    (Character|StopJumping)))

(event EventBeginPlay
  (bind _asplayer_controller (Utilities|Casting|CastToPlayerController (Pawn|GetController)))
  (Utilities|IsValid (PlayerController|LocalPlayerSubsystems|GetEnhancedInputLocalPlayerSubsystem _asplayer_controller)
    (:Is%20Valid
      (Input|AddMappingContext (PlayerController|LocalPlayerSubsystems|GetEnhancedInputLocalPlayerSubsystem _asplayer_controller) "/Game/2dPlatformer/Input/IMC_GAME.IMC_GAME" 0 "(bIgnoreAllPressedKeysUntilRelease=True,bForceImmediately=False,bNotifyUserSettings=False)"))))

(event EventTick
  (params (DeltaSeconds :type Float%20%28single-precision%29))
  (bind _sprite (Variables|Default|GetSprite))
  (bind _charactermovement (Variables|Character|GetCharacterMovement))
  (bind _velocity (Variables|/Script/Engine.MovementComponent|GetVelocity _charactermovement))
  (Pawn|Input|AddMovementInput (Math|Vector|MakeVector (Variables|Default|GettargetXVelocity) 0.0 0.0) 1.0 false)
  (Sprite|SetFlipbook _sprite (select (!= (.z _velocity) 0.0) (select (> (.z _velocity) 0.0) "/Game/2dPlatformer/Art/Character/Character_VelocityManager/FB_Jump.FB_Jump" "/Game/2dPlatformer/Art/Character/Character_VelocityManager/FB_Fall2.FB_Fall2") (select (!= (.x _velocity) 0.0) "/Game/2dPlatformer/Art/Character/Character_Move/Move.Move" "/Game/2dPlatformer/Art/Character/Character_idle/Idle.Idle")))
  (Transformation|SetRelativeRotation _sprite (Math|Rotator|SelectRotator "0.000000,0.000000,0.000000" "0.000000,180.000000,0.000000" (> (.x (Variables|/Script/Engine.MovementComponent|GetVelocity (Variables|Character|GetCharacterMovement))) 0.0)) false false))

(fn ConstructionScript)