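; BP_Ghost is a flying ghost character for the 2D platformer that homes in on the player.
; Each tick it forces Flying movement mode and checks whether the player is within RangeToTrack.
; In range, it sets target X and Z velocities from the normalized direction to the player; otherwise both are zero.
; It then calls the parent Tick, with no code here applying those velocities itself.
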(event EventBeginPlay
  (|CallParentFunction) ; This node is disabled and will not be called.\nDrag off pins to build functionality.
)

(event EventTick
  (params (DeltaSeconds :type Float%20%28single-precision%29))
  (bind _returnvalue (Game|GetPlayerCharacter 0))
  (bind _self self)
  (bind _returnvalue_2 (Transformation|GetActorLocation _self))
  (bind _returnvalue_3 (Transformation|GetActorLocation _returnvalue))
  (bind _returnvalue_4 (- _returnvalue_3 _returnvalue_2))
  (bind _returnvalue_5 (Math|Vector|Normalize _returnvalue_4))
  (Pawn|Components|CharacterMovement|SetMovementMode (Variables|Character|GetCharacterMovement) "MOVE_Flying" 0)
  (bind _istrue (CallFunction|InRangeOfPlayer (Variables|Default|GetrangeToTrack)))
  (Variables|Default|SettargetXVelocity (Math|Float|SelectFloat (.x _returnvalue_5) 0.0 _istrue))
  (Variables|Default|SettargetZVelocity (Math|Float|SelectFloat (.z _returnvalue_5) 0.0 _istrue))
  (|CallParentFunction DeltaSeconds))

(fn ConstructionScript
  (|CallParentFunction))