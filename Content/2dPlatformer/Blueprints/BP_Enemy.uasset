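; BP_Enemy is a 2D platformer enemy that damages the player whenever they come within attack range.
; Each Tick runs AttackPlayer, which lazily caches the BP_Player reference, compares distance to AttackRange and passes the enemy's location to the player's Damage, with no cooldown here.
; Tick and construction also call the parent class.
; A separate InRangeOfPlayer helper tests player distance against a given range but is not called in this graph.
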(event EventBeginPlay)

(event Collision|EventActorBeginOverlap
  (params (OtherActor :type Actor%20Object%20Reference)))

(event EventTick
  (params (DeltaSeconds :type Float%20%28single-precision%29))
  (CallFunction|AttackPlayer)
  (|CallParentFunction 0.0))

(fn ConstructionScript
  (|CallParentFunction))

(fn InRangeOfPlayer
  (params (Range :type Float%20%28double-precision%29))
  (return (> Range (Math|Vector|Distance(Vector) (Transformation|GetActorLocation (Game|GetPlayerCharacter 0)) (Transformation|GetActorLocation self)))))

(fn AttackPlayer
  (if (Utilities|IsValid (LocalVariables|GetPlayer))
    _
    (else
      (bind _asbp_player (Utilities|Casting|CastToBP_Player (Game|GetPlayerCharacter 0)))
      (bind _output_get (LocalVariables|SetPlayer _asbp_player))))
  (if (<= (Math|Vector|Distance(Vector) (Transformation|GetActorLocation (LocalVariables|GetPlayer)) (Transformation|GetActorLocation)) (Variables|Default|GetattackRange))
    (Default|Damage _output_get (Transformation|GetActorLocation))))