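; 2D platformer zombie character that patrols by reversing its horizontal direction at ledges and walls.
; Each tick, a single offset line trace, mirrored by TargetXVelocity, flips that value when it finds nothing or hits within DistanceToWall.
; Tick also swaps the sprite between move and idle flipbooks based on actual X velocity.
; Movement input is not applied here, only the target direction is set.
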(event EventTick
  (params (DeltaSeconds :type Float%20%28single-precision%29))
  (bind _charactermovement (Variables|Character|GetCharacterMovement))
  (bind _velocity (Variables|/Script/Engine.MovementComponent|GetVelocity _charactermovement))
  (CallFunction|HandleAnimation (.x _velocity) (.z _velocity))
  (CallFunction|CheckforFloorandWalls)
  (|CallParentFunction DeltaSeconds))

(event EventBeginPlay
  (Variables|Default|SettargetXVelocity 1.0)
  (|CallParentFunction))

(fn ConstructionScript
  (|CallParentFunction))

(fn CheckforFloorandWalls
  (bind _returnvalue (Transformation|GetActorLocation))
  (bind _offset (Variables|Default|Getoffset))
  (bind (_outhit _returnvalue_2) (Collision|LineTraceForObjects _returnvalue (+ _returnvalue (Math|Vector|MakeVector (* (.x _offset) (Variables|Default|GettargetXVelocity)) (.y _offset) (.z _offset))) (LocalVariables|GetLayerCheck) false 0 "None" true "(R=1.000000,G=0.000000,B=0.000000,A=1.000000)" "(R=0.000000,G=1.000000,B=0.000000,A=1.000000)" 0.1))
  (Variables|Default|SettargetXVelocity (Math|Float|SelectFloat (* (Variables|Default|GettargetXVelocity) -1.0) (Variables|Default|GettargetXVelocity) (or (<= (.distance _outhit) (LocalVariables|GetdistanceToWall)) (not _returnvalue_2))))
  (return))

(fn HandleAnimation
  (params (xVelocity :type Float%20%28double-precision%29) (zVelocity :type Float%20%28double-precision%29))
  (LocalVariables|SetxVel xVelocity)
  (LocalVariables|SetzVel zVelocity)
  (Sprite|SetFlipbook (Variables|Default|GetSprite) (select (!= (LocalVariables|GetxVel) 0.0) "/Game/2dPlatformer/Art/Zombie/Zombie_Move/Zombie_Move.Zombie_Move" "/Game/2dPlatformer/Art/Zombie/Zombie_Idle/Zombie_Idle.Zombie_Idle")))