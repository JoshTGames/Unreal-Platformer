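; 2D platformer character Blueprint with movement, sprite flipping, sliding, wall hang and wall jump.
; Tick applies Slide every frame, caching then overriding friction, braking, capsule height and sprite offset, or restoring the cached values.
; When not sliding, it applies target movement, yaws the sprite to face travel and runs Climb.
; Climb line-traces along horizontal input to zero velocity on walls, and launches away when HandleJump's flag is set during a hang.
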(event EventTick
  (params (DeltaSeconds :type Float%20%28single-precision%29))
  (bind _doslide (Variables|Default|GetdoSlide))
  (CallFunction|Slide _doslide)
  (if (not _doslide)
    (Pawn|Input|AddMovementInput (Math|Vector|MakeVector (Variables|Default|GettargetXVelocity) 0.0 (Variables|Default|GettargetZVelocity)) 1.0 false)
    (CallFunction|RotateSprite)
    (CallFunction|Climb)))

(fn ConstructionScript)

(fn Slide
  (params (doSlide :type Boolean))
  (bind _charactermovement (Variables|Character|GetCharacterMovement))
  (bind _capsulecomponent (Variables|Collision|GetCapsuleComponent))
  (bind _sprite (Variables|Default|GetSprite))
  (bind _charactermovement_2 (Variables|Character|GetCharacterMovement))
  (if doSlide
    (LocalVariables|Setfriction (Variables|/Script/Engine.CharacterMovementComponent|GetGroundFriction _charactermovement_2))
    (LocalVariables|SetbreakingSpeed (Variables|/Script/Engine.CharacterMovementComponent|GetBrakingDecelerationWalking _charactermovement_2))
    (LocalVariables|SetcollisionSize (Variables|/Script/Engine.CapsuleComponent|GetCapsuleHalfHeight _capsulecomponent))
    (LocalVariables|SetspritePosition (.z (Variables|/Script/Engine.SceneComponent|GetRelativeLocation _sprite)))
    (Variables|/Script/Engine.CharacterMovementComponent|SetGroundFriction _charactermovement_2 0.0)
    (Variables|/Script/Engine.CharacterMovementComponent|SetBrakingDecelerationWalking _charactermovement_2 64.0)
    (Components|Capsule|SetCapsuleHalfHeight _capsulecomponent 4.0 true)
    (Transformation|SetRelativeLocation _sprite (Math|Vector|MakeVector 0.0 0.0 1.9) false false)
    (else
      (Variables|/Script/Engine.CharacterMovementComponent|SetGroundFriction _charactermovement (LocalVariables|Getfriction))
      (Variables|/Script/Engine.CharacterMovementComponent|SetBrakingDecelerationWalking _charactermovement (LocalVariables|GetbreakingSpeed))
      (Components|Capsule|SetCapsuleHalfHeight (Variables|Collision|GetCapsuleComponent) (LocalVariables|GetcollisionSize) true)
      (Transformation|SetRelativeLocation _sprite (Math|Vector|MakeVector 0.0 0.0 (LocalVariables|GetspritePosition)) false false))))

(fn Climb
  (bind _returnvalue (Transformation|GetActorLocation))
  (bind _walljumpforce (Variables|Default|GetwallJumpForce))
  (if (Variables|Default|GetisJumping)
    (if (Variables|Default|GetwallHang)
      (Variables|Default|SetwallHang false)
      (Variables|/Script/Engine.MovementComponent|SetVelocity (Variables|Character|GetCharacterMovement) (Math|Vector|MakeVector (/ (* (* (Variables|Default|GettargetXVelocity) -1.0) _walljumpforce) 2.0) 0.0 _walljumpforce)))
    (else
      (bind _returnvalue_2 (Collision|LineTraceByChannel _returnvalue (+ _returnvalue (Math|Vector|MakeVector (* (Variables|Default|GettargetXVelocity) (Variables|Default|GetwallCheckLength)) 0.0 0.0)) "TraceTypeQuery1" false 0 "None"))
      (Variables|/Script/Engine.MovementComponent|SetVelocity (Variables|Character|GetCharacterMovement) (Math|Vector|SelectVector "0, 0, 0" (Variables|/Script/Engine.MovementComponent|GetVelocity (Variables|Character|GetCharacterMovement)) _returnvalue_2))
      (Variables|Default|SetwallHang _returnvalue_2))))

(fn HandleJump
  (params (isJumping :type Boolean))
  (bind _output_get (Variables|Default|SetisJumping isJumping))
  (if _output_get
    (Character|Jump)
    (else
      (Character|StopJumping))))

(fn RotateSprite
  (bind _targetxvelocity (Variables|Default|GettargetXVelocity))
  (bind _returnvalue (Math|Float|NormalizetoRange _targetxvelocity -1e+02 1e+02))
  (Transformation|SetRelativeRotation (Variables|Default|GetSprite) (Math|Rotator|MakeRotator 0.0 0.0 (Math|Float|SelectFloat (.yaw (Variables|/Script/Engine.SceneComponent|GetRelativeRotation (Variables|Default|GetSprite))) (Math|Conversions|ToFloat(Integer) (* (- 1 (Math|Float|Round _returnvalue)) 180)) (== _returnvalue 0.5))) false false))